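; Actor that starts and stops Take Recorder captures by gloss name and reports their status to web endpoints.
; startRecord records via the Take Recorder panel, then sends take path and name by HTTP GET to a remote worker URL.
; stopRecord ends recording, notifies localhost, loops playback of the sequence and calls an export trigger after a delay.
; Mesh-repositioning logic exists but is never run.
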(event `start Record`
  (params (glosName :type Text))
  (set `self.glosName` (`KismetTextLibrary.Conv_TextToString` glosName))
  ;[1 1 1] Fetch recorder start recording
  (bind _returnvalue (`self.FetchTakeRecordStartRecording`))
  ;[1 1 1] Msg that we are recording
  (`self.MsgRecording` (`TakeRecorder.GetSequence` _returnvalue) (`KismetTextLibrary.Conv_TextToString` glosName)))

(event `stop Record`
  (params (glosName :type Text))
  (`KismetSystemLibrary.PrintText` glosName)
  (set `self.glosName` (`KismetTextLibrary.Conv_TextToString` glosName))
  ;[1 1 1] Stop Take Recorder if it is Running
  (if (`TakeRecorderBlueprintLibrary.IsRecording`)
    (`TakeRecorderBlueprintLibrary.StopRecording`)
    (bind _returnvalue (`TakeRecorder.GetSequence` (stale `start Record` _returnvalue)))
    (bind (_outactor _returnvalue_2) (`LevelSequencePlayer.CreateLevelSequencePlayer` _returnvalue))
    (set `self.levelSeqeuncerName` _returnvalue)
    ;[1 1 1] Msg that we stop recording
    (`self.MsgStopRecording` (`KismetSystemLibrary.GetPathName` _returnvalue) (`self.glosName`))
    ;[1 1 1] Loop replay and set locations
    (`MovieSceneSequencePlayer.PlayLooping` (`LevelSequenceActor.SequencePlayer` _outactor) 3)
    (message `AnimationDataModel.GetAnimationSequence` _returnvalue)
    (set `self.NewVar_1` (`MovieSceneSequencePlayer.GetSequenceName` _returnvalue_2 true))
    (`KismetSystemLibrary.PrintString` "Hello")
    (`KismetSystemLibrary.Delay` 5.0)
    (`self.TriggerExport`)))

(fn `FetchAndSetLocation`
  (bind _returnvalue (`SceneComponent.K2_GetComponentLocation` (`self.Masculine_TPose_characterized`)))
  ;[1 1 1] Fetch and set play location
  (`KismetSystemLibrary.PrintText` (`KismetTextLibrary.Conv_VectorToText` _returnvalue) true true (struct :`G` 0.66 :`B` 1.0 :`A` 1.0) 100.0)
  (set `self.NewVar_2` _returnvalue)
  (bind _output_get (set `self.wereldLocatie` (0.0 0.0 500.0)))
  (`SceneComponent.K2_SetWorldLocation` (`self.Masculine_TPose_characterized`) _output_get false false))

(fn `FetchTakeRecordStartRecording`
  (returns (ReturnValue :type "TakeRecorder Object Reference"))
  ;[1 1 1] Fetch Take record and start recording
  (bind _returnvalue (`TakeRecorderBlueprintLibrary.OpenTakeRecorderPanel`))
  (bind _returnvalue_2 (`TakeRecorderBlueprintLibrary.GetDefaultParameters`))
  (message `AnimationDataModel.GetAnimationSequence` _returnvalue)
  (`TakeRecorderPanel.SetupForRecording_TakePreset` (`TakeRecorderBlueprintLibrary.GetTakeRecorderPanel`) null)
  (bind _returnvalue_3 (`TakeRecorderBlueprintLibrary.StartRecording` (`TakeRecorderPanel.GetLevelSequence` _returnvalue) (`TakeRecorderPanel.GetSources` _returnvalue) (`TakeRecorderPanel.GetTakeMetaData` _returnvalue) _returnvalue_2))
  (return _returnvalue_3))

(fn `MsgRecording`
  (params (Object :type "Object Object Reference") (Value :type String))
  ;[1 1 1] MsgWeAreRecording
  (`MasterHttpRequestBPLibrary.MasterRequestWithPayloadAndHeaders` "https://leffe.science.uva.nl:8043/ue_worker.php" "GET" (`|MakeArray` (struct) :!type "KeyValuePair Structure") (`|MakeArray` (make `KeyValuePair` "Status" "IsPlaying") (make `KeyValuePair` "Take" (`KismetSystemLibrary.GetPathName` Object)) (make `KeyValuePair` "glosName" Value))))

(fn `MsgStopRecording`
  (params (Value :type String) (Value2 :type String))
  ;[1 1 1] Msg Stop recording
  (`MasterHttpRequestBPLibrary.MasterRequestWithPayloadAndHeaders` "http://localhost:3000?status=isrecording" "GET" (`|MakeArray` (struct) :!type "KeyValuePair Structure") (`|MakeArray` (make `KeyValuePair` "Status" "Stopped") (make `KeyValuePair` "Take" Value) (make `KeyValuePair` "glosName" Value2))))

(fn `UserConstructionScript`)